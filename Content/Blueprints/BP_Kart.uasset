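; BP_Kart is a modular kart actor that assembles its visual parts from mesh and location variables on BeginPlay.
; It sets meshes and relative offsets for body, spoiler, four wheels and light, deriving each wheel pair from one offset by negating X.
; It then sets its world Z to the negated front wheel Z offset, keeping X and Y.
; The construction script is empty, and the file contains no driving logic.
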(event EventBeginPlay
  (bind _returnvalue (Transformation|GetActorLocation))
  (bind _light (Variables|Default|GetLight))
  (bind _wheelsfrontloc (Variables|Default|GetWheelsFrontLoc))
  (bind _wheelrearloc (Variables|Default|GetWheelRearLoc))
  (bind _spoiler (Variables|Default|GetSpoiler))
  (bind _wheelfrontleft (Variables|Default|GetWheelFrontLeft))
  (bind _wheelfrontright (Variables|Default|GetWheelFrontRight))
  (bind _wheelrearleft (Variables|Default|GetWheelRearLeft))
  (bind _wheelrearright (Variables|Default|GetWheelRearRight))
  (bind _body (Variables|Default|GetBody))
  (Components|StaticMesh|SetStaticMesh _body (Variables|Default|GetBodyMesh))
  (Transformation|SetRelativeLocation _body (Variables|Default|GetBodyLoc) false false)
  (Components|StaticMesh|SetStaticMesh _spoiler (Variables|Default|GetSpoilerMesh))
  (Transformation|SetRelativeLocation _spoiler (Variables|Default|GetSpoilerLoc) false false)
  (Components|StaticMesh|SetStaticMesh _wheelfrontleft (Variables|Default|GetWheelsLeftMesh))
  (Transformation|SetRelativeLocation _wheelfrontleft (Variables|Default|GetWheelsFrontLoc) false false)
  (Components|StaticMesh|SetStaticMesh _wheelfrontright (Variables|Default|GetWheelsRightMesh))
  (Transformation|SetRelativeLocation _wheelfrontright (Math|Vector|MakeVector (* (.x _wheelsfrontloc) -1.0) (.y _wheelsfrontloc) (.z _wheelsfrontloc)) false false)
  (Components|StaticMesh|SetStaticMesh _wheelrearleft (Variables|Default|GetWheelsLeftMesh))
  (Transformation|SetRelativeLocation _wheelrearleft (Math|Vector|MakeVector (* (.x _wheelrearloc) -1.0) (.y _wheelrearloc) (.z _wheelrearloc)) false false)
  (Components|StaticMesh|SetStaticMesh _wheelrearright (Variables|Default|GetWheelsRightMesh))
  (Transformation|SetRelativeLocation _wheelrearright (Variables|Default|GetWheelRearLoc) false false)
  (Components|StaticMesh|SetStaticMesh _light (Variables|Default|GetLightMesh))
  (Transformation|SetRelativeLocation _light (Variables|Default|GetLightLoc) false false)
  (Transformation|SetActorLocation (Math|Vector|MakeVector (.x _returnvalue) (.y _returnvalue) (* (.z (Variables|Default|GetWheelsFrontLoc)) -1.0)) false false))

(event Collision|EventActorBeginOverlap
  (params (OtherActor :type Actor%20Object%20Reference)))

(event EventTick
  (params (DeltaSeconds :type Float%20%28single-precision%29)))

(fn ConstructionScript)