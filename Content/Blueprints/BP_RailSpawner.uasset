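; BP_RailSpawner is a placed marker that spawns straight two-point BP_Rail connections between paired spawners at game start.
; Spawners pair by signed ID: on BeginPlay, each positive-ID instance searches all spawners for those with the matching negative ID.
; For each match it spawns a BP_Rail at its own location, then rebuilds the rail's spline and stretches its spline mesh to the partner's relative position.
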(event EventBeginPlay
  (bind _returnvalue (Math|Vector|MakeVector 0.0 0.0 0.0))
  (bind _returnvalue_2 (Transformation|GetActorLocation))
  (if (> (Variables|Default|GetID) 0)
    (bind _outactors (Actor|GetAllActorsOfClass "BP_RailSpawner_C"))
    (for _array_element _outactors
      (if (== (Variables|BP_RailSpawner_C|GetID _array_element) (* (Variables|Default|GetID) -1))
        (bind _returnvalue_3 (Game|SpawnActorfromClass "/Game/Blueprints/BP_Rail.BP_Rail_C" (Math|Transform|MakeTransform "0, 0, 0" "0, 0, 0" "1.000000,1.000000,1.000000") "Undefined" "MultiplyWithRoot" 0 0))
        (Transformation|SetActorLocation _returnvalue_3 _returnvalue_2 false false)
        (Spline|ClearSplinePoints (Variables|/Game/Blueprints/BP_Rail.BP_Rail_C|GetSpline _returnvalue_3) true)
        (Spline|AddSplinePoint (Variables|/Game/Blueprints/BP_Rail.BP_Rail_C|GetSpline _returnvalue_3) _returnvalue "Local" true)
        (Spline|AddSplinePoint (Variables|/Game/Blueprints/BP_Rail.BP_Rail_C|GetSpline _returnvalue_3) (+ _returnvalue (- (Transformation|GetActorLocation _array_element) _returnvalue_2)) "Local" true)
        (SplineMesh|SetStartandEnd (Variables|/Game/Blueprints/BP_Rail.BP_Rail_C|GetSplineMesh _returnvalue_3) _returnvalue _returnvalue (+ _returnvalue (- (Transformation|GetActorLocation _array_element) _returnvalue_2)) (+ _returnvalue (- (Transformation|GetActorLocation _array_element) _returnvalue_2)) true :!class /Script/Engine.SplineMeshComponent)))))

(event Collision|EventActorBeginOverlap
  (params (OtherActor :type Actor%20Object%20Reference)))

(event EventTick
  (params (DeltaSeconds :type Float%20%28single-precision%29)))

(fn ConstructionScript)