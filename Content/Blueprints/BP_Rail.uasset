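; BP_Rail is a rail actor that builds a row of repeated static meshes when play begins.
; BeginPlay divides the spline length by Spacing, floored at 1, and adds a Static Mesh component with the assigned Mesh at each step.
; Pieces advance along local X with a fixed 90-degree rotation, so the spline sets only their count, not their path.
; The construction script is empty.
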(event EventBeginPlay
  (bind _output_get (Variables|Default|SetCount (Math|Float|Truncate (/ (Spline|GetSplineLength (Variables|Default|GetSpline)) (Math|Float|Max(Float) (Variables|Default|GetSpacing) 1.0)))))
  (for _index (range 0 _output_get)
    (bind _returnvalue (AddComponent|AddStaticMeshComponent false (Math|Transform|MakeTransform (Math|Vector|MakeVector (* (Variables|Default|GetSpacing) _index) 0.0 0.0) "0.000000,90.000000,0.000000" "1.000000,1.000000,1.000000")))
    (Components|StaticMesh|SetStaticMesh _returnvalue (Variables|Default|GetMesh))))

(event Collision|EventActorBeginOverlap
  (params (OtherActor :type Actor%20Object%20Reference)))

(event EventTick
  (params (DeltaSeconds :type Float%20%28single-precision%29)))

(fn ConstructionScript)